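; BP_Player is the player character Blueprint, handling Enhanced Input setup and movement.
; BeginPlay adds IMC_Player_Controller to the owning player controller's input subsystem.
; IA_Move feeds movement along the full control rotation's right and forward vectors, without isolating yaw.
; It also stores the axes in SideInput and ForwardInput, zeroing both when input completes.
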(event Input|EnhancedActionEvents|EnhancedInputActionIA_Move
  (params (ActionValue :type Vector%202D%20Structure) (ElapsedSeconds :type Float%20%28double-precision%29) (TriggeredSeconds :type Float%20%28double-precision%29) (InputAction :type Input%20Action%20Object%20Reference :default "/Game/ARProject/Controller/InputAction/IA_Move.IA_Move"))
  (bind _returnvalue (Pawn|GetControlRotation :!class /Script/Engine.Pawn))
  ;[1 1 1] Move
  (:Triggered
    (Variables|Default|SetSide_input (.x ActionValue))
    (Variables|Default|SetForward_input (.y ActionValue))
    (Pawn|Input|AddMovementInput (Math|Vector|GetRightVector _returnvalue) (Variables|Default|GetSide_input) false)
    (Pawn|Input|AddMovementInput (Math|Vector|GetForwardVector _returnvalue) (Variables|Default|GetForward_input) false))
  (:Completed
    (Variables|Default|SetSide_input 0.0)
    (Variables|Default|SetForward_input 0.0)))

(event EventBeginPlay
  ;[1 1 1] Input Mapping
  (bind _as플레이어_컨트롤러 (Utilities|Casting|CastToPlayerController (Pawn|GetController)))
  (Utilities|IsValid _as플레이어_컨트롤러
    (:Is%20Valid
      (Input|AddMappingContext (PlayerController|LocalPlayerSubsystems|GetEnhancedInputLocalPlayerSubsystem _as플레이어_컨트롤러) "/Game/ARProject/Controller/IMC_Player_Controller.IMC_Player_Controller" 0 "(bIgnoreAllPressedKeysUntilRelease=True,bForceImmediately=False,bNotifyUserSettings=False)"))))

(event Collision|EventActorBeginOverlap
  (params (OtherActor :type Actor%20Object%20Reference)))

(event EventTick
  (params (DeltaSeconds :type Float%20%28single-precision%29)))

(fn ConstructionScript)